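; BP_OurGameMode is a game mode that runs a countdown timer and tracks score for a water-depositing game.
; The timer starts from an initial value, counts down each tick and shows on screen through a keyed debug print string until it reaches zero and flags the game as ended.
; A WaterDeposited event adds bonus time and score.
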(event Custom|WaterDeposited
  (params (TimeGained :type Float%20%28double-precision%29) (ScoreGained :type Integer))
  (Variables|Default|SetTimeRemaining (+ (Variables|Default|GetTimeRemaining) TimeGained))
  (Variables|Default|SetScore (+ (Variables|Default|GetScore) ScoreGained)))

(event EventBeginPlay
  (Variables|Default|SetTimeRemaining (Variables|Default|GetInitialTime)))

(event EventTick
  (params (DeltaSeconds :type Float%20%28single-precision%29))
  (if (not (Variables|Default|GetHasGameEnded))
    (bind _output_get (Variables|Default|SetTimeRemaining (- (Variables|Default|GetTimeRemaining) DeltaSeconds)))
    (if (<= _output_get 0.0)
      (Variables|Default|SetHasGameEnded true)
      (else
        (Development|PrintString (Utilities|String|Append "Time Remaining: " (Utilities|String|ToString(Float) (Variables|Default|GetTimeRemaining))) true false "(R=0.000000,G=0.660000,B=1.000000,A=1.000000)" 2.0 "Timer")))))

(fn ConstructionScript)