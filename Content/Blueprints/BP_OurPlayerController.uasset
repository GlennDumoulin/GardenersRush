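; Player controller that turns Enhanced Input movement into world-space movement input for player pawn 0.
; BeginPlay adds the IMC_Input mapping context.
; Tick polls IA_Movement, swaps its axes, clamps the vector's length and, when non-zero, passes it to AddMovementInput scaled by delta time and MovementSpeed.
; Disconnected leftover logic for consuming input, offsetting the pawn and smoothly rotating it toward its movement direction never runs.
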(event EventBeginPlay
  (bind _returnvalue (PlayerController|LocalPlayerSubsystems|GetEnhancedInputLocalPlayerSubsystem))
  (Utilities|IsValid _returnvalue
    (:Is%20Valid
      (Input|AddMappingContext _returnvalue "/Game/Blueprints/Input/IMC_Input.IMC_Input" 0 "(bIgnoreAllPressedKeysUntilRelease=True,bForceImmediately=False)"))))

(event EventTick
  (params (DeltaSeconds :type Float%20%28single-precision%29))
  (bind _returnvalue (Input|EnhancedActionValues|GetIA_Movement))
  (bind _returnvalue_2 (Math|Vector|MakeVector (.y _returnvalue) (.x _returnvalue) 0.0))
  (bind _returnvalue_3 (Math|Vector|ClampVectorSize _returnvalue_2 0.0 1.0))
  (if (> (Math|Vector|VectorLengthSquared _returnvalue_3) 0.0)
    (Pawn|Input|AddMovementInput (Game|Player|GetPlayerPawn 0) (* (* DeltaSeconds _returnvalue_3) (Variables|Default|GetMovementSpeed)) 1.0 false)))

(fn ConstructionScript)