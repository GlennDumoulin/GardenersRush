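; Puddle actor that offers itself to the gardener character as an interactable object through a Box overlap.
; Any begin overlap sets IsNearPlayer, then, if the player controller reports IsStarted, assigns the puddle to the overlapping BP_NewGardener's IntercatableObject.
; The gardener leaving the box clears that reference and the flag.
; The interaction itself is not implemented here, and a debug print remains after the controller cast.
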(event OnComponentBeginOverlap(Box)
  (params (OverlappedComponent :type Primitive%20Component%20Object%20Reference) (OtherActor :type Actor%20Object%20Reference) (OtherComp :type Primitive%20Component%20Object%20Reference) (OtherBodyIndex :type Integer) (bFromSweep :type Boolean) (SweepResult :type Hit%20Result%20Structure%20%28by%20ref%29))
  (Variables|Default|SetIsNearPlayer true)
  (bind _asbp_our_player_controller (Utilities|Casting|CastToBP_OurPlayerController (Game|GetPlayerController 0)))
  (Development|PrintString "cast succeeded")
  (if (Variables|/Game/Blueprints/BP_OurPlayerController.BP_OurPlayerController_C|GetIsStarted _asbp_our_player_controller)
    (bind _asbp_new_gardener (Utilities|Casting|CastToBP_NewGardener OtherActor))
    (Variables|/Game/Blueprints/BP_NewGardener.BP_NewGardener_C|SetIntercatableObject _asbp_new_gardener self)))

(event OnComponentHit(Cube)
  (params (HitComponent :type Primitive%20Component%20Object%20Reference) (OtherActor :type Actor%20Object%20Reference) (OtherComp :type Primitive%20Component%20Object%20Reference) (NormalImpulse :type Vector :default "0, 0, 0") (Hit :type Hit%20Result%20Structure%20%28by%20ref%29)))

(event OnComponentEndOverlap(Box)
  (params (OverlappedComponent :type Primitive%20Component%20Object%20Reference) (OtherActor :type Actor%20Object%20Reference) (OtherComp :type Primitive%20Component%20Object%20Reference) (OtherBodyIndex :type Integer))
  (bind _asbp_new_gardener (Utilities|Casting|CastToBP_NewGardener OtherActor))
  (Variables|/Game/Blueprints/BP_NewGardener.BP_NewGardener_C|SetIntercatableObject _asbp_new_gardener 0)
  (Variables|Default|SetIsNearPlayer false))

(event OnComponentHit(Box)
  (params (HitComponent :type Primitive%20Component%20Object%20Reference) (OtherActor :type Actor%20Object%20Reference) (OtherComp :type Primitive%20Component%20Object%20Reference) (NormalImpulse :type Vector :default "0, 0, 0") (Hit :type Hit%20Result%20Structure%20%28by%20ref%29)))

(event EventBeginPlay)

(event Collision|EventActorBeginOverlap
  (params (OtherActor :type Actor%20Object%20Reference)))

(event EventTick
  (params (DeltaSeconds :type Float%20%28single-precision%29)))

(fn ConstructionScript)